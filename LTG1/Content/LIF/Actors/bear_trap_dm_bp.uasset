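; Bear trap actor that hurts the first-person player on contact until a shot disables it.
; While intact, each overlap subtracts DivisionesAReducir from the character's Health and sets its SANGREX flag.
; A hit from a FirstPersonProjectile turns on physics for the struck component and sets Destruida, which stops further damage without removing the actor.
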(event EventBeginPlay)

(event Collision|EventActorBeginOverlap
  (params (OtherActor :type Actor%20Object%20Reference))
  ;[1 1 1] DAÑAR PERSONAJE SIN DESTRUIR LA TRAMPA
  (bind _asfirst_person_character (Utilities|Casting|CastToFirstPersonCharacter OtherActor))
  (if (not (Variables|Default|GetDestruida))
    (Variables|/Game/FirstPersonBP/Blueprints/FirstPersonCharacter.FirstPersonCharacter_C|SetHealth _asfirst_person_character (- (Variables|/Game/FirstPersonBP/Blueprints/FirstPersonCharacter.FirstPersonCharacter_C|GetHealth _asfirst_person_character) (Variables|Default|GetDivisionesAReducir)))
    (Variables|/Game/FirstPersonBP/Blueprints/FirstPersonCharacter.FirstPersonCharacter_C|SetSANGRE_X _asfirst_person_character true)))

(event Collision|EventHit
  (params (MyComp :type Primitive%20Component%20Object%20Reference) (Other :type Actor%20Object%20Reference) (OtherComp :type Primitive%20Component%20Object%20Reference) (bSelfMoved :type Boolean) (HitLocation :type Vector :default "0, 0, 0") (HitNormal :type Vector :default "0, 0, 0") (NormalImpulse :type Vector :default "0, 0, 0") (Hit :type Hit%20Result%20Structure%20%28by%20ref%29))
  ;[1 1 1] DESTRUIR LA TRAMPA SOLO AL RECIBIR UN DISPARO
  (Utilities|Casting|CastToFirstPersonProjectile Other)
  (Physics|SetSimulatePhysics MyComp true)
  (Variables|Default|SetDestruida true))

(fn ConstructionScript)